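; Main level-flow Blueprint that scripts the intro title, background music and commandant Levchenko's radio dialogue.
; BeginPlay locks movement until the title ends, loops shuffled async-loaded music, and plays a title animation when the gate opens.
; TookWrench starts subtitled voiceovers; Gate nodes fed by Answer repeat the knock prompt until acknowledged, then branch on yes/no into a briefing about Uncle Styopa or the elevator objective.
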(event Custom|TitleEnd_Event
  (Input|SetIgnoreMoveInput (Game|GetPlayerController 0) false))

(event Custom|OnObjectStateChangedDelegate_Event
  (params (NewState :type Gameplay%20Tag%20Structure))
  (bind _titles (Variables|Default|GetTitles))
  (if (== NewState "(TagName=\"CIS.Gate.Opened\")")
    (UserInterface|Animation|PlayAnimation _titles (Variables|/Game/ProjectDyadyaStyopa/UI/WBP_BeginTitle.WBP_BeginTitle_C|GetSetTitle _titles) 0.0 1 "Forward" 1.0 false)))

(event EventBeginPlay
  (Utilities|FlowControl|Sequence
    (:then_0
      (Input|SetIgnoreMoveInput (Game|GetPlayerController 0) true)
      (bind _returnvalue (UserInterface|CreateWidget "/Game/ProjectDyadyaStyopa/UI/WBP_BeginTitle.WBP_BeginTitle_C" (Game|GetPlayerController 0)))
      (Variables|Default|SetTitles _returnvalue)
      (UserInterface|Viewport|AddtoViewport _returnvalue 0)
      (EventDispatchers|AssignTitleEnd _returnvalue (delegate Custom|TitleEnd_Event)))
    (:then_1
      (Utilities|Array|Shuffle (Variables|Default|GetOST) :!label _label)
      (bind _object (Utilities|AsyncLoadAsset (Utilities|Array|Get(acopy) (Variables|Default|GetOST)))
        (:Completed
          (bind _assound_cue (Utilities|Casting|CastToSoundCue _object))
          (Audio|PlaySound2D _assound_cue 1.0 1.0 0.0 0 0)
          (Utilities|FlowControl|Delay (Variables|/Script/Engine.SoundBase|GetDuration _assound_cue))
          (goto _label))))
    (:then_2
      (bind _object_2 (Utilities|AsyncLoadAsset (Variables|Default|GetGate))
        (:Completed
          (bind _asbp_gate (Utilities|Casting|CastToBP_Gate _object_2))
          (EventDispatchers|AssignOnObjectStateChangedDelegate (Variables|/Game/CharacterInteraction/Blueprints/InteractionObjects/BP_BaseInteractObject.BP_BaseInteractObject_C|GetCISInteractionObject _asbp_gate) (delegate Custom|OnObjectStateChangedDelegate_Event)))))))

(event EventAnswer
  (params (Yes/No :type Boolean))
  (Utilities|FlowControl|Sequence
    (:then_0
      (if Yes/No
        (Utilities|FlowControl|Sequence
          (:then_0
            (Utilities|FlowControl|Gate true
              (:Exit
                (bind _duration (CallFunction|PlayVoiceoverandSubtitle "Слышу вас, отлично. Прежде чем двинуться дальше, дайте мне знать: осведомлены ли вы о месте, куда попали, и что здесь происходит? Если да, стукните два раза по трубе. Если нет, один раз. Это важно для вашей безопасности и дальнейших действий." "/Game/ProjectDyadyaStyopa/Audio/ElevenLabs_2024-03-11T23_29_57_Jake_-_Realistic_Hard_Working_gen_s50_sb75_se0_b_m2_Cue.ElevenLabs_2024-03-11T23_29_57_Jake_-_Realistic_Hard_Working_gen_s50_sb75_se0_b_m2_Cue" "0, 0, 0" 0 0 false 1.0))
                (Utilities|FlowControl|Delay _duration)
                (goto _label Open))))
          (:then_1
            (Utilities|FlowControl|DoOnce false
              (:Completed
                (Utilities|FlowControl|Gate false) ; enters at Close
              ))))))
    (:then_1
      (Utilities|FlowControl|Gate true :!label _label
        (:Exit
          (if Yes/No
            (Utilities|FlowControl|DoOnce false
              (:Completed
                (bind _duration_2 (CallFunction|PlayVoiceoverandSubtitle "Понимаю, вы решили не вдаваться в подробности. В любом случае, ваша главная задача остаётся неизменной — добраться до лифта. Он находится в конце главного коридора и сейчас заблокирован. Если удастся его разблокировать, вы сможете покинуть этот комплекс и помочь мне и оставшимся выжившим. Будьте очень внимательны и осторожны на своём пути." "/Game/ProjectDyadyaStyopa/Audio/ElevenLabs_2024-03-11T23_30_47_Jake_-_Realistic_Hard_Working_gen_s50_sb75_se0_b_m2_Cue.ElevenLabs_2024-03-11T23_30_47_Jake_-_Realistic_Hard_Working_gen_s50_sb75_se0_b_m2_Cue" "0, 0, 0" 0 0 false 1.0))
                (Utilities|FlowControl|Delay _duration_2)))
            (else
              (Utilities|FlowControl|DoOnce false
                (:Completed
                  (bind _duration_3 (CallFunction|PlayVoiceoverandSubtitle "Хорошо, позвольте уточнить. Ситуация такова: проект \"Дядя Стёпа\" полностью вышел из-под контроля. Большая часть сотрудников базы погибла. Местоположение объекта \"Дядя Стёпа\" в данный момент неустановлено. Он может находиться где угодно внутри комплекса. Вместе со мной здесь небольшая группа сотрудников, которые также выжили. Мы все в ловушке и нуждаемся в помощи. Ваша задача — пройти к лифту через главный коридор, разблокировать его и помочь нам эвакуироваться. Будьте настороже, двигаясь по базе." "/Game/ProjectDyadyaStyopa/Audio/ElevenLabs_2024-03-11T23_31_37_Jake_-_Realistic_Hard_Working_gen_s50_sb75_se0_b_m2_Cue.ElevenLabs_2024-03-11T23_31_37_Jake_-_Realistic_Hard_Working_gen_s50_sb75_se0_b_m2_Cue" "0, 0, 0" 0 0 false 1.0))
                  (Utilities|FlowControl|Delay _duration_3))))))))))

(event EventTookWrench
  (bind _duration (CallFunction|PlayVoiceoverandSubtitle "Здесь комендант Левченко, местоположение - котельная. Визуальный и аудио контакт невозможен, связь односторонняя через этот громкоговоритель. Если вы меня слышите, прошу откликнуться, ударив два раза по любой трубе." "/Game/ProjectDyadyaStyopa/Audio/ElevenLabs_2024-03-11T23_28_57_Jake_-_Realistic_Hard_Working_gen_s50_sb75_se0_b_m2_Cue.ElevenLabs_2024-03-11T23_28_57_Jake_-_Realistic_Hard_Working_gen_s50_sb75_se0_b_m2_Cue" "0, 0, 0" 0 0 false 1.0))
  (Utilities|FlowControl|Delay _duration)
  (Utilities|FlowControl|Sequence
    (:then_0
      (Utilities|FlowControl|Delay 1e+01)
      (Utilities|FlowControl|Gate false :!label _label
        (:Exit
          (bind _duration_2 (CallFunction|PlayVoiceoverandSubtitle "Это комендант Левченко ещё раз. Если мои слова до вас дошли, дайте знать - дважды стукните по трубе." "/Game/ProjectDyadyaStyopa/Audio/ElevenLabs_2024-03-11T23_29_32_Jake_-_Realistic_Hard_Working_gen_s50_sb75_se0_b_m2_Cue.ElevenLabs_2024-03-11T23_29_32_Jake_-_Realistic_Hard_Working_gen_s50_sb75_se0_b_m2_Cue" "0, 0, 0" 0 0 false 1.0))
          (Utilities|FlowControl|Delay _duration_2)
          (goto _label))))
    (:then_1
      (Utilities|FlowControl|Gate true) ; enters at Open
    )))

(fn ConstructionScript)