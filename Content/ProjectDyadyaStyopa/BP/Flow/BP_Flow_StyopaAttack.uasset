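; Flow Blueprint that runs Styopa's attack as an ending sequence when a trigger box is overlapped.
; It async-loads the referenced trigger and binds a one-shot overlap handler, which async-loads the Styopa skeletal mesh actor.
; Styopa's animation plays with an attached roar; after the animation's length, the roar stops, a final cue plays and the ending title widget appears.
; After a delay, it opens the main map.
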(event Custom|OnActorBeginOverlap_Event
  (params (OverlappedActor :type Actor%20Object%20Reference) (OtherActor :type Actor%20Object%20Reference))
  (Utilities|FlowControl|DoOnce false
    (:Completed
      (bind _object (Utilities|AsyncLoadAsset (Variables|Default|GetStyopa))
        (:Completed
          (bind _asskeletal_mesh_actor (Utilities|Casting|CastToSkeletalMeshActor _object))
          (Audio|Components|Audio|Play (Variables|/Script/Engine.SkeletalMeshActor|GetSkeletalMeshComponent _asskeletal_mesh_actor) false)
          (bind _returnvalue (Audio|SpawnSoundAttached "/Game/Zombie/Sound/Entity/SC_Entity_Roar.SC_Entity_Roar" (Variables|/Script/Engine.SkeletalMeshActor|GetSkeletalMeshComponent _asskeletal_mesh_actor) "None" "0, 0, 0" "0, 0, 0" "KeepRelativeOffset" false 1.0 1.0 0.0 0 0))
          (Utilities|FlowControl|Delay (Animation|GetPlayLength (.AnimToPlay (Utilities|Struct|BreakSingleAnimationPlayData (Variables|/Script/Engine.SkeletalMeshComponent|GetAnimationData (Variables|/Script/Engine.SkeletalMeshActor|GetSkeletalMeshComponent _asskeletal_mesh_actor))))))
          (Audio|SpawnSoundAttached "/Game/HorrorSoundPack/Audio/Cue/fin2_Cue.fin2_Cue" (Variables|/Script/Engine.SkeletalMeshActor|GetSkeletalMeshComponent _asskeletal_mesh_actor) "None" "0, 0, 0" "0, 0, 0" "KeepRelativeOffset" false 1.0 1.0 0.0 0 0)
          (bind _returnvalue_2 (UserInterface|CreateWidget "/Game/ProjectDyadyaStyopa/UI/WBP_FinTitle.WBP_FinTitle_C" (Game|GetPlayerController 0)))
          (UserInterface|Viewport|AddtoViewport _returnvalue_2 0)
          (Audio|Components|Audio|Stop _returnvalue)
          (Utilities|FlowControl|Delay 1e+01)
          (Game|OpenLevel(byObjectReference) "/Game/ProjectDyadyaStyopa/Maps/MainMap.MainMap"))))))

(event EventBeginPlay
  (bind _object (Utilities|AsyncLoadAsset (Variables|Default|GetStyopaTrigger))
    (:Completed
      (bind _astrigger_box (Utilities|Casting|CastToTriggerBox _object))
      (EventDispatchers|AssignOnActorBeginOverlap _astrigger_box (delegate Custom|OnActorBeginOverlap_Event)))))

(fn ConstructionScript)