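; BP_Flow_Wrench is a one-shot, box-triggered scripted scare built around a skeletal mesh actor placed in the level.
; On overlap it async-loads the soft-referenced actor and plays a zombie roar at its location.
; A second later it plays the LS_Flow_Wrench sequence, flings the mesh by a pelvis impulse and plays a cue cut after three seconds.
; It then reveals hidden decals and destroys the referenced ambient actor and itself.
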(event OnComponentBeginOverlap(Box)
  (params (OverlappedComponent :type Primitive%20Component%20Object%20Reference) (OtherActor :type Actor%20Object%20Reference) (OtherComp :type Primitive%20Component%20Object%20Reference) (OtherBodyIndex :type Integer) (bFromSweep :type Boolean) (SweepResult :type Hit%20Result%20Structure%20%28by%20ref%29))
  (Utilities|FlowControl|DoOnce false
    (:Completed
      (bind _object (Utilities|AsyncLoadAsset (Variables|Default|GetSkeletalMesh))
        (:Completed
          (bind _asskeletal_mesh_actor (Utilities|Casting|CastToSkeletalMeshActor _object))
          (Audio|SpawnSoundatLocation "/Game/Zombie/Sound/Zombie/Roar/S_Zombie_Roar_C.S_Zombie_Roar_C" (Transformation|GetWorldLocation (Variables|/Script/Engine.SkeletalMeshActor|GetSkeletalMeshComponent _asskeletal_mesh_actor)) "0, 0, 0" 1.0 1.0 0.0 0 0)
          (Utilities|FlowControl|Delay 1.0)
          (bind _returnvalue (Sequencer|Player|CreateLevelSequencePlayer "/Game/ProjectDyadyaStyopa/LS_Flow_Wrench.LS_Flow_Wrench"))
          (Sequencer|Player|Play _returnvalue :!class /Script/MovieScene.MovieSceneSequencePlayer)
          (Physics|AddImpulse (Variables|/Script/Engine.SkeletalMeshActor|GetSkeletalMeshComponent _asskeletal_mesh_actor) "0.000000,-187500.000000,0.000000" "Pelvis" false)
          (bind _returnvalue_2 (Audio|SpawnSoundatLocation "/Game/HorrorSoundPack/Audio/Cue/finz_Cue.finz_Cue" (Transformation|GetWorldLocation (Variables|/Script/Engine.SkeletalMeshActor|GetSkeletalMeshComponent _asskeletal_mesh_actor)) "0, 0, 0" 0.7 1.0 0.0 0 0))
          (Audio|Components|Audio|StopDelayed _returnvalue_2 3.0)
          (for _array_element (Variables|Default|GetDecals)
            (Rendering|SetActorHiddenInGame (Utilities|ResolveSoftReference _array_element) false))
          (Actor|DestroyActor (Utilities|ResolveSoftReference (Variables|Default|GetAmbient))))))))

(fn ConstructionScript)