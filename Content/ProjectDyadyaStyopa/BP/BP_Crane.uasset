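; Crane actor that drops and replaces a suspended physics box in response to a switch.
; It listens to the state delegate of a child-actor BP_SimpleSwitcher, branching on the CIS button gameplay tag.
; Switch on breaks the physics constraint and nudges the original Box downward.
; Switch off adds a new heavy simulated mesh copying Box's mesh and constrains it to the Crane, without removing earlier boxes.
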(event Custom|OnObjectStateChangedDelegate_Event
  (params (NewState :type Gameplay%20Tag%20Structure))
  (|SwitchGameplayTag NewState
    (:CIS.Button.SwitchOn
      (Class|PhysicsConstraintComponent|BreakConstraint (Variables|Default|GetPhysicsConstraint))
      (Physics|AddImpulse (Variables|Default|GetBox) "0.000000,0.000000,-1.000000" "None" false))
    (:CIS.Button.SwitchOff
      (bind _returnvalue (AddComponent|AddStaticMeshComponent false (Math|Transform|MakeTransform "77.000000,0.000000,-485.000000" "0, 0, 0" "1.000000,1.000000,1.000000")))
      (Components|StaticMesh|SetStaticMesh _returnvalue (Variables|/Script/Engine.StaticMeshComponent|GetStaticMesh (Variables|Default|GetBox)))
      (Physics|SetSimulatePhysics _returnvalue true)
      (Class|PrimitiveComponent|SetMassOverrideinKg _returnvalue "None" 2e+03 true)
      (Class|PhysicsConstraintComponent|SetConstrainedComponents (Variables|Default|GetPhysicsConstraint) (Variables|Default|GetCrane) "None" _returnvalue "None"))))

(event EventBeginPlay
  (bind _asbp_simple_switcher (Utilities|Casting|CastToBP_SimpleSwitcher (Variables|/Script/Engine.ChildActorComponent|GetChildActor (Variables|Default|GetChildActor))))
  (EventDispatchers|AssignOnObjectStateChangedDelegate (Variables|/Game/CharacterInteraction/Blueprints/InteractionObjects/BP_BaseInteractObject.BP_BaseInteractObject_C|GetCISInteractionObject _asbp_simple_switcher) (delegate Custom|OnObjectStateChangedDelegate_Event)))

(fn ConstructionScript)