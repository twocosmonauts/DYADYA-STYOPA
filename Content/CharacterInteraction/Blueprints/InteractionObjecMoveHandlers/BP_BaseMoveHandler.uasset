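; Base move handler that brings a BP_CISCharacter into position and orientation for interacting with an object.
; Root-motion flying move runs toward GetMoveLocation while tick rotates the character and first-person camera, finishing when both movement and rotation complete.
; Afterwards, the local first-person camera briefly holds the pitch-clamped look point, then optionally levels out.
; Target location and rotation getters return zero placeholders, apparently for child handlers to override.
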(event EventMovementAborted
  (params (InteractionCharacter :type Character%20Object%20Reference) (CharacterInteractionComponent :type CIS%20Character%20Interaction%20Component%20Object%20Reference) (InteractionObjectComponent :type CIS%20Interaction%20Object%20Component%20Object%20Reference) (InteractionObjectSide :type CIS%20Interaction%20Object%20Side%20Structure%20%28by%20ref%29))
  (bind _movetask (Variables|Internal|GetMoveTask)
    (:then
      (Class|CISRootMotionMovementTask|FinishMovement _movetask))
    (:else)))

(event EventHandlerTick
  (params (DeltaTime :type Float%20%28single-precision%29) (InteractionCharacter :type Character%20Object%20Reference) (CharacterInteractionComponent :type CIS%20Character%20Interaction%20Component%20Object%20Reference) (InteractionObjectComponent :type CIS%20Interaction%20Object%20Component%20Object%20Reference) (InteractionObjectSide :type CIS%20Interaction%20Object%20Side%20Structure%20%28by%20ref%29))
  (bind _tpcharacter (Variables|Internal|GetTPCharacter))
  (bind _tpcharacter_2 (Variables|Internal|GetTPCharacter))
  (bind _returnvalue (Pawn|GetControlRotation _tpcharacter :!class /Script/Engine.Pawn))
  (Variables|Internal|SetDeltaTime DeltaTime)
  (if (not (Class|CISInteractionObjectMoveHandler|IsMovementFinished))
    (bind _done (CallFunction|RotateCharacter DeltaTime))
    (if (and _done (Variables|Internal|GetMovementToLocationFinished))
      (Class|CISInteractionObjectMoveHandler|FinishMovement)
      (Variables|Internal|SetTimeAfterFinishMovement (Utilities|Time|GetTimeSeconds self)))
    (elif (Pawn|IsLocallyControlled (Variables|Internal|GetTPCharacter))
      (bind _tpcharacter_3 (Variables|Internal|GetTPCharacter)
        (:then
          (if (Variables|/Game/CharacterInteraction/Blueprints/BP_CISCharacter.BP_CISCharacter_C|GetFirstPerson _tpcharacter_3)
            (if (and (Variables|Settings|ReturnCamera|GetNeedReturnCameraRotation) (> (- (Utilities|Time|GetTimeSeconds self) (Variables|Internal|GetTimeAfterFinishMovement)) (Variables|Settings|ReturnCamera|GetStartReturnCameraTime)))
              (Pawn|SetControlRotation (Pawn|GetController _tpcharacter) (Math|Interpolation|RInterpTo _returnvalue (Math|Rotator|MakeRotator 0.0 0.0 (.Yaw (Math|Rotator|BreakRotator _returnvalue))) (Variables|Internal|GetDeltaTime) (Variables|Settings|ReturnCamera|GetReturnCameraSpeed)))
              (elif (< (- (Utilities|Time|GetTimeSeconds self) (Variables|Internal|GetTimeAfterFinishMovement)) (Variables|Settings|GetLookPointFocusTime))
                (bind _tpcharacter_4 (Variables|Internal|GetTPCharacter)
                  (:then
                    (if (Variables|/Game/CharacterInteraction/Blueprints/BP_CISCharacter.BP_CISCharacter_C|GetFirstPerson _tpcharacter_4)
                      (Pawn|SetControlRotation (Pawn|GetController _tpcharacter_2) (Math|Interpolation|RInterpTo (Pawn|GetControlRotation _tpcharacter_2 :!class /Script/Engine.Pawn) (CallFunction|GetClampedRotationtoLookPoint) (Variables|Internal|GetDeltaTime) (Variables|Settings|GetCameraRotationSpeed)))))
                  (:else))))))
        (:else)))))

(event EventStartMovement
  (params (InteractionCharacter :type Character%20Object%20Reference) (CharacterInteractionComponent :type CIS%20Character%20Interaction%20Component%20Object%20Reference) (InteractionObjectComponent :type CIS%20Interaction%20Object%20Component%20Object%20Reference) (InteractionObjectSide :type CIS%20Interaction%20Object%20Side%20Structure%20%28by%20ref%29))
  (bind _returnvalue (Components|GetOwner InteractionObjectComponent))
  (Variables|Internal|SetMovementToLocationFinished false)
  (bind _asbp_cischaracter (Utilities|Casting|CastToBP_CISCharacter InteractionCharacter)
    (:then
      (Variables|Internal|SetTPCharacter _asbp_cischaracter)
      (Variables|Internal|SetInteractObjectActor (Components|GetOwner InteractionObjectComponent))
      (Variables|Internal|SetLookPointComponent (.ReturnValue (Class|CISFunctionLibrary|GetSceneComponentwithName _returnvalue (Variables|Settings|GetLookingPoint))))
      (Variables|Internal|SetMoveComponent (.ReturnValue (Class|CISFunctionLibrary|GetSceneComponentwithName _returnvalue (Variables|Settings|GetMoveToThisComponent))))
      (bind _task (|RootMotionMoveto (Variables|Internal|GetTPCharacter) (CallFunction|GetMoveLocation) "ECC_WorldStatic" 0.0 "MOVE_Flying" "Override" false 0.0 1.0 -15.0)
        (:OnRootMotionMovementCreated
          (Variables|Internal|SetMoveTask _task))
        (:OnRootMotionMovementFinished
          (Variables|Internal|SetMovementToLocationFinished true :!label _label))
        (:OnTimeOut
          (goto _label))))
    (:CastFailed
      (Class|CISInteractionObjectMoveHandler|FinishMovement))))

(fn RotateCharacter
  (params (DeltaTime :type Float%20%28double-precision%29))
  (bind _tpcharacter (Variables|Internal|GetTPCharacter))
  (Transformation|SetActorRotation (Variables|Internal|GetTPCharacter) (Class|KismetMathLibrary|RInterptoConstant (Transformation|GetActorRotation (Variables|Internal|GetTPCharacter)) (CallFunction|GetCharacterRotation) DeltaTime (Variables|Settings|GetCharacterRotationSpeed)))
  (LocalVariables|SetCharacterRotationDone (Math|Rotator|Equal(Rotator) (Transformation|GetActorRotation (Variables|Internal|GetTPCharacter)) (CallFunction|GetCharacterRotation) 0.1))
  (if (Variables|/Game/CharacterInteraction/Blueprints/BP_CISCharacter.BP_CISCharacter_C|GetFirstPerson (Variables|Internal|GetTPCharacter))
    (if (Pawn|IsLocallyControlled (Variables|Internal|GetTPCharacter))
      (Pawn|SetControlRotation (Pawn|GetController _tpcharacter) (Math|Interpolation|RInterpTo (Pawn|GetControlRotation _tpcharacter :!class /Script/Engine.Pawn) (CallFunction|GetClampedRotationtoLookPoint) DeltaTime (Variables|Settings|GetCameraRotationSpeed)))
      (return (and (LocalVariables|GetCharacterRotationDone) (Math|Rotator|Equal(Rotator) (Pawn|GetControlRotation (Variables|Internal|GetTPCharacter) :!class /Script/Engine.Pawn) (CallFunction|GetClampedRotationtoLookPoint) 2.0)))
      (else
        (return false)))
    (else
      (return (LocalVariables|GetCharacterRotationDone)))))

(fn GetMoveLocation
  (return "0, 0, 0"))

(fn GetCharacterRotation
  (return (Math|Rotator|MakeRotator 0.0 0.0 0.0)))

(fn GetRotationtoLookPoint
  (return (Math|Rotator|MakeRotator 0.0 0.0 0.0)))

(fn GetLookPointLocation
  (bind _lookpointcomponent (Variables|Internal|GetLookPointComponent)
    (:then
      (return (Transformation|GetWorldLocation _lookpointcomponent)))
    (:else)))

(fn GetClampedRotationtoLookPoint
  (bind _rotation (CallFunction|GetRotationtoLookPoint))
  (bind _self self)
  (bind _returnvalue (Game|GetPlayerCameraManager _self))
  (if (Pawn|IsLocallyControlled (Variables|Internal|GetTPCharacter))
    (return (Math|Rotator|MakeRotator (.roll _rotation) (Math|Float|Clamp(Float) (.pitch _rotation) (Variables|/Script/Engine.PlayerCameraManager|GetViewPitchMin _returnvalue) (Variables|/Script/Engine.PlayerCameraManager|GetViewPitchMax _returnvalue)) (.yaw _rotation)))
    (else
      (return (CallFunction|GetRotationtoLookPoint)))))