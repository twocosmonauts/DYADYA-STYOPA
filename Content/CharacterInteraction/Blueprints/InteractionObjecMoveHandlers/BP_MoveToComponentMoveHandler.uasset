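; BP_MoveToComponentMoveHandler is a character interaction move handler that uses a MoveComponent's transform as the character's move target.
; The component's world location and rotation supply the move location and character rotation.
; The look rotation takes its pitch from the character's spring arm toward the look point, keeps the component's yaw and zeroes roll.
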(fn GetMoveLocation
  (return (Transformation|GetWorldLocation (Variables|Default|GetMoveComponent))))

(fn GetCharacterRotation
  (return (Transformation|GetWorldRotation (Variables|Default|GetMoveComponent))))

(fn GetRotationtoLookPoint
  (return (Math|Rotator|MakeRotator 0.0 (.pitch (Math|Rotator|FindLookatRotation (Transformation|GetWorldLocation (Variables|/Game/CharacterInteraction/Blueprints/BP_CISCharacter.BP_CISCharacter_C|GetSpringArm (Variables|Default|GetTPCharacter))) (CallFunction|GetLookPointLocation))) (.yaw (Transformation|GetWorldRotation (Variables|Default|GetMoveComponent))))))