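; Interaction move handler that positions the player character at a set MoveDistance from a named component on the interact object.
; The move target lies on the 2D line from that component's socket toward the character, keeping the character's current Z.
; Character yaw looks from the character toward MoveComponent.
; Look rotation reuses that yaw and takes pitch from the spring arm toward the look point.
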(fn GetMoveLocation
  (bind _tpcharacter (Variables|Default|GetTPCharacter))
  (bind _movetothiscomponent (Variables|Default|GetMoveToThisComponent))
  (bind _interactobjectactor (Variables|Default|GetInteractObjectActor))
  (bind _interactobjectactor_2 (Variables|Default|GetInteractObjectActor))
  (bind _movedistance (Variables|Settings|GetMoveDistance))
  (bind _movetothiscomponent_2 (Variables|Default|GetMoveToThisComponent))
  (bind _socketlocation (Class|CISFunctionLibrary|GetSceneComponentwithName _interactobjectactor_2 _movetothiscomponent))
  (bind _returnvalue (Transformation|GetActorLocation _tpcharacter))
  (bind _socketlocation_2 (Class|CISFunctionLibrary|GetSceneComponentwithName _interactobjectactor _movetothiscomponent_2))
  (bind _returnvalue_2 (Math|Conversions|ToVector2D(Vector) _socketlocation))
  (bind _returnvalue_3 (Math|Conversions|ToVector2D(Vector) _returnvalue))
  (bind _returnvalue_4 (Math|Conversions|ToVector2D(Vector) _socketlocation_2))
  (bind _returnvalue_5 (- _returnvalue_3 _returnvalue_2))
  (bind _returnvalue_6 (Math|Vector2D|Normalize2D _returnvalue_5))
  (bind _returnvalue_7 (* _returnvalue_6 _movedistance))
  (bind _returnvalue_8 (+ _returnvalue_4 _returnvalue_7))
  (return (Math|Vector|MakeVector (.x _returnvalue_8) (.y _returnvalue_8) (.z (Transformation|GetActorLocation (Variables|Default|GetTPCharacter))))))

(fn GetCharacterRotation
  (return (Math|Rotator|MakeRotator 0.0 0.0 (.yaw (Math|Rotator|FindLookatRotation (Transformation|GetActorLocation (Variables|Default|GetTPCharacter)) (Transformation|GetWorldLocation (Variables|Default|GetMoveComponent)))))))

(fn GetRotationtoLookPoint
  (return (Math|Rotator|MakeRotator 0.0 (.pitch (Math|Rotator|FindLookatRotation (Transformation|GetWorldLocation (Variables|/Game/CharacterInteraction/Blueprints/BP_CISCharacter.BP_CISCharacter_C|GetSpringArm (Variables|Default|GetTPCharacter))) (CallFunction|GetLookPointLocation))) (.yaw (CallFunction|GetCharacterRotation)))))