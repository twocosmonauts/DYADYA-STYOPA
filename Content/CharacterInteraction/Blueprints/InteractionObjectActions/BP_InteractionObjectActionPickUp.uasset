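; Interaction object action that plays a character pick-up montage suited to the height of the object being interacted with.
; GetPickUpAnim picks from the PickUpMontages map the montage whose height value is nearest the absolute vertical offset between the capsule bottom and the object.
; A timer set to the duration returned by PlayAnimMontage finishes the action.
; Interruption clears that timer and stops the character's current montage.
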(event Custom|FinishActionTimer
  (Class|CISInteractionObjectAction|FinishAction))

(event Custom|SetFinishTimer
  (params (Time :type Float%20%28double-precision%29))
  (bind _returnvalue (Utilities|Time|SetTimerbyEvent (delegate Custom|FinishActionTimer) Time))
  (Variables|Internal|SetTimerHandle _returnvalue))

(event EventStartInteractionObjectAction
  (params (InteractionCharacter :type Character%20Object%20Reference) (CharacterInteractionComponent :type CIS%20Character%20Interaction%20Component%20Object%20Reference) (InteractionObjectComponent :type CIS%20Interaction%20Object%20Component%20Object%20Reference) (InteractionObjectSide :type CIS%20Interaction%20Object%20Side%20Structure%20%28by%20ref%29))
  (bind _returnvalue (Animation|PlayAnimMontage InteractionCharacter (CallFunction|GetPickUpAnim InteractionCharacter (Components|GetOwner InteractionObjectComponent)) 1.0 "None"))
  (CallFunction|SetFinishTimer _returnvalue))

(event EventOnUseFinished
  (params (InteractionCharacter :type Character%20Object%20Reference) (CharacterInteractionComponent :type CIS%20Character%20Interaction%20Component%20Object%20Reference) (InteractionObjectComponent :type CIS%20Interaction%20Object%20Component%20Object%20Reference) (bWasInterrupted :type Boolean))
  (if bWasInterrupted
    (Utilities|Time|ClearandInvalidateTimerbyHandle InteractionCharacter (Variables|Internal|GetTimerHandle))
    (Animation|StopAnimMontage InteractionCharacter (Animation|GetCurrentMontage InteractionCharacter :!class /Script/Engine.Character))))

(fn GetPickUpAnim
  (params (Character :type Character%20Object%20Reference) (PickObject :type Actor%20Object%20Reference))
  (bind _values (Utilities|Map|Values (Variables|Settings|GetPickUpMontages)))
  (for (_array_element _array_index) _values
    (if (< (Math|Float|Absolute(Float) (- _array_element (Math|Float|Absolute(Float) (.z (- (- (Transformation|GetActorLocation Character) (Math|Vector|MakeVector 0.0 0.0 (Components|Capsule|GetScaledCapsuleHalfHeight (Variables|/Script/Engine.Character|GetCapsuleComponent Character)))) (Transformation|GetActorLocation PickObject)))))) (LocalVariables|GetNearestDistance))
      (LocalVariables|SetNearestDistance (Math|Float|Absolute(Float) (- _array_element (Math|Float|Absolute(Float) (.z (- (- (Transformation|GetActorLocation Character) (Math|Vector|MakeVector 0.0 0.0 (Components|Capsule|GetScaledCapsuleHalfHeight (Variables|/Script/Engine.Character|GetCapsuleComponent Character)))) (Transformation|GetActorLocation PickObject)))))))
      (LocalVariables|SetIndex _array_index)))
  (bind _keys (Utilities|Map|Keys (Variables|Settings|GetPickUpMontages)))
  (return (Utilities|Array|Get(acopy) _keys (LocalVariables|GetIndex))))