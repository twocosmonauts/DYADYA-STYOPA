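; Interaction object action that plays a montage on the interacting character and, optionally, a second montage on a named skeletal mesh of the interacted object.
; A timer finishes the action, timed just short of the object montage's length when one is set, otherwise to the character montage's duration.
; On interruption, it stops the object's montage, clears the timer and stops the character's montage, all dependent on finding that skeletal mesh.
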(event Custom|FinishActionTimer
  (Class|CISInteractionObjectAction|FinishAction))

(event Custom|SetFinishTimer
  (params (Time :type Float%20%28double-precision%29))
  (bind _returnvalue (Utilities|Time|SetTimerbyEvent (delegate Custom|FinishActionTimer) Time))
  (Variables|Internal|SetTimerHandle _returnvalue))

(event EventStartInteractionObjectAction
  (params (InteractionCharacter :type Character%20Object%20Reference) (CharacterInteractionComponent :type CIS%20Character%20Interaction%20Component%20Object%20Reference) (InteractionObjectComponent :type CIS%20Interaction%20Object%20Component%20Object%20Reference) (InteractionObjectSide :type CIS%20Interaction%20Object%20Side%20Structure%20%28by%20ref%29))
  (bind _returnvalue (Animation|PlayAnimMontage InteractionCharacter (Variables|Settings|GetMontageOnCharacter) 1.0 "None"))
  (Variables|Settings|GetMontageOnObject
    (:then
      (bind _asskeletal_mesh_component (Utilities|Casting|CastToSkeletalMeshComponent (.ReturnValue (Class|CISFunctionLibrary|GetPrimitiveComponentwithName (Components|GetOwner InteractionObjectComponent) (Variables|Settings|GetMeshComponentOnObject)))))
      (Utilities|FlowControl|Sequence
        (:then_0
          (Animation|Montage|PlayMontage _asskeletal_mesh_component (Variables|Settings|GetMontageOnObject)))
        (:then_1
          (CallFunction|SetFinishTimer (- (Variables|/Script/Engine.AnimSequenceBase|GetSequenceLength (Variables|Settings|GetMontageOnObject)) 0.05)))))
    (:else
      (CallFunction|SetFinishTimer _returnvalue))))

(event EventOnUseFinished
  (params (InteractionCharacter :type Character%20Object%20Reference) (CharacterInteractionComponent :type CIS%20Character%20Interaction%20Component%20Object%20Reference) (InteractionObjectComponent :type CIS%20Interaction%20Object%20Component%20Object%20Reference) (bWasInterrupted :type Boolean))
  (if bWasInterrupted
    (bind _asskeletal_mesh_component (Utilities|Casting|CastToSkeletalMeshComponent (.ReturnValue (Class|CISFunctionLibrary|GetPrimitiveComponentwithName (Components|GetOwner InteractionObjectComponent) (Variables|Settings|GetMeshComponentOnObject)))))
    (Animation|Montage|MontageStop (Components|SkeletalMesh|GetAnimInstance _asskeletal_mesh_component) 0.2 (Animation|Montage|GetCurrentActiveMontage (Components|SkeletalMesh|GetAnimInstance _asskeletal_mesh_component)))
    (Utilities|Time|ClearandInvalidateTimerbyHandle InteractionCharacter (Variables|Internal|GetTimerHandle))
    (Animation|StopAnimMontage InteractionCharacter (Animation|GetCurrentMontage InteractionCharacter :!class /Script/Engine.Character))))