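; BP_CodeLockAction is an interaction object action that lets the player character operate a code lock.
; On start it caches the player controller and the owning BP_CodeLock, binds to the lock's finish-use dispatcher, starts its use and enables input on the lock actor.
; The Finish event unbinds that dispatcher, disables the lock's input and completes the action.
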(event Custom|Finish
  (bind _codelock (Variables|Default|GetCodeLock))
  (EventDispatchers|UnbindallEventsfromDFinishUse _codelock)
  (Input|DisableInput _codelock (Variables|Default|GetPC))
  (Class|CISInteractionObjectAction|FinishAction))

(event EventStartInteractionObjectAction
  (params (InteractionCharacter :type Character%20Object%20Reference) (CharacterInteractionComponent :type CIS%20Character%20Interaction%20Component%20Object%20Reference) (InteractionObjectComponent :type CIS%20Interaction%20Object%20Component%20Object%20Reference) (InteractionObjectSide :type CIS%20Interaction%20Object%20Side%20Structure%20%28by%20ref%29))
  (bind _returnvalue (Components|GetOwner InteractionObjectComponent))
  (Utilities|Casting|CastToBP_CISCharacter InteractionCharacter)
  (bind _asplayer_controller (Utilities|Casting|CastToPlayerController (Pawn|GetController InteractionCharacter)))
  (Variables|Default|SetPC _asplayer_controller)
  (bind _asbp_code_lock (Utilities|Casting|CastToBP_CodeLock _returnvalue))
  (Variables|Default|SetCodeLock _asbp_code_lock)
  (EventDispatchers|AssignDFinishUse _asbp_code_lock (EventDispatchers|CreateEvent :!event Custom|Finish))
  (Default|OnStartUse (Variables|Default|GetCodeLock))
  (Input|EnableInput _returnvalue _asplayer_controller))