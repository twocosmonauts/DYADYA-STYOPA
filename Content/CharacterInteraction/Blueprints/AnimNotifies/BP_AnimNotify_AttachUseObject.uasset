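; Anim notify state that attaches the character's currently used interaction object to the animated mesh for the span of the notify.
; On begin, it gets the owner's CISCharacterInteractionComponent and attaches the using object's owner to a configurable socket, snapping location and rotation while keeping world scale.
; On end, it hides that actor in game without detaching it.
; Only the interaction component is validity-checked, not the used object.
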(fn ReceivedNotifyBegin
  (params (MeshComp :type Skeletal%20Mesh%20Component%20Object%20Reference) (Animation :type Anim%20Sequence%20Base%20Object%20Reference) (TotalDuration :type Float%20%28single-precision%29) (EventReference :type Anim%20Notify%20Event%20Reference%20Structure%20%28by%20ref%29))
  (bind _returnvalue (Components|GetOwner MeshComp))
  (bind _returnvalue_2 (Actor|GetComponentbyClass _returnvalue "/Script/CharacterInteractionSystem.CISCharacterInteractionComponent"))
  (Utilities|IsValid _returnvalue_2
    (:Is%20Valid
      (Transformation|AttachComponentToComponent (Components|GetOwner (Class|CISCharacterInteractionComponent|GetCurrentUsingObject _returnvalue_2)) MeshComp (Variables|Default|GetSocketName) "SnapToTarget" "SnapToTarget" "KeepWorld" true)
      (return false))
    (:Is%20Not%20Valid
      (return false))))

(fn ReceivedNotifyEnd
  (params (MeshComp :type Skeletal%20Mesh%20Component%20Object%20Reference) (Animation :type Anim%20Sequence%20Base%20Object%20Reference) (EventReference :type Anim%20Notify%20Event%20Reference%20Structure%20%28by%20ref%29))
  (bind _returnvalue (Components|GetOwner MeshComp))
  (bind _returnvalue_2 (Actor|GetComponentbyClass _returnvalue "/Script/CharacterInteractionSystem.CISCharacterInteractionComponent"))
  (Utilities|IsValid _returnvalue_2
    (:Is%20Valid
      (Rendering|SetActorHiddenInGame (Components|GetOwner (Class|CISCharacterInteractionComponent|GetCurrentUsingObject _returnvalue_2)) true)
      (return true))
    (:Is%20Not%20Valid
      (return false))))