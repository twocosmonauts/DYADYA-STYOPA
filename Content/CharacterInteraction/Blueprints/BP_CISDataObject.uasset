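; Data object for the Character Interaction System that links an interactable's state to its on-screen widget and to the character using it.
; Overlap toggles the owning BP_BaseInteractObject's widget component active, and visibility changes show or hide its prompt.
; Best-object and usability changes mark the widget usable only when this object is the character's best candidate.
; During use, character movement is disabled and the capsule ignores WorldDynamic and Pawn, both restored on finish.
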(event Custom|UpdateUsable
  (bind _cachedinteractionobjectcomponent (Variables|Default|GetCachedInteractionObjectComponent)
    (:then
      (bind _asbp_base_interact_object (Utilities|Casting|CastToBP_BaseInteractObject (Components|GetOwner _cachedinteractionobjectcomponent)))
      (Default|Usable (Default|GetInteractionWidget _asbp_base_interact_object) (== (Variables|/Script/CharacterInteractionSystem.CISCharacterInteractionComponent|GetBestObjectToUse (Variables|Default|GetCachedCharacterInteractionComponent)) (Variables|Default|GetCachedInteractionObjectComponent))))
    (:else)))

(event Custom|OnBestObjectForUseChangedDelegate_Event
  (params (InteractionObjectComponent :type CIS%20Interaction%20Object%20Component%20Object%20Reference))
  (CallFunction|UpdateUsable))

(event EventOnMovementEnded
  (params (Character :type Character%20Object%20Reference) (CharacterInteractionComponent :type CIS%20Character%20Interaction%20Component%20Object%20Reference) (InteractionObjectComponent :type CIS%20Interaction%20Object%20Component%20Object%20Reference)))

(event EventOnMovementStarted
  (params (Character :type Character%20Object%20Reference) (CharacterInteractionComponent :type CIS%20Character%20Interaction%20Component%20Object%20Reference) (InteractionObjectComponent :type CIS%20Interaction%20Object%20Component%20Object%20Reference)))

(event EventOnObjectActionStarted
  (params (Action :type CIS%20Interaction%20Object%20Action%20Object%20Reference) (Character :type Character%20Object%20Reference) (CharacterInteractionComponent :type CIS%20Character%20Interaction%20Component%20Object%20Reference) (InteractionObjectComponent :type CIS%20Interaction%20Object%20Component%20Object%20Reference)))

(event EventOnObjectUseFinished
  (params (Character :type Character%20Object%20Reference) (CharacterInteractionComponent :type CIS%20Character%20Interaction%20Component%20Object%20Reference) (InteractionObjectComponent :type CIS%20Interaction%20Object%20Component%20Object%20Reference) (bInterrupted :type Boolean))
  (bind _capsulecomponent (Variables|/Script/Engine.Character|GetCapsuleComponent Character))
  (bind _asbp_cischaracter (Utilities|Casting|CastToBP_CISCharacter Character))
  (Default|DisableMovement _asbp_cischaracter false)
  (Collision|SetCollisionResponsetoChannel _capsulecomponent "ECC_WorldDynamic" "ECR_Block")
  (Collision|SetCollisionResponsetoChannel _capsulecomponent "ECC_Pawn" "ECR_Block"))

(event EventOnObjectUseStarted
  (params (Character :type Character%20Object%20Reference) (CharacterInteractionComponent :type CIS%20Character%20Interaction%20Component%20Object%20Reference) (InteractionObjectComponent :type CIS%20Interaction%20Object%20Component%20Object%20Reference))
  (bind _capsulecomponent (Variables|/Script/Engine.Character|GetCapsuleComponent Character))
  (bind _asbp_cischaracter (Utilities|Casting|CastToBP_CISCharacter Character))
  (Default|DisableMovement _asbp_cischaracter true)
  (Collision|SetCollisionResponsetoChannel _capsulecomponent "ECC_WorldDynamic" "ECR_Ignore")
  (Collision|SetCollisionResponsetoChannel _capsulecomponent "ECC_Pawn" "ECR_Ignore"))

(event EventOnUsableChanged
  (params (Character :type Character%20Object%20Reference) (CharacterInteractionComponent :type CIS%20Character%20Interaction%20Component%20Object%20Reference) (InteractionObjectComponent :type CIS%20Interaction%20Object%20Component%20Object%20Reference) (bUsable :type Boolean))
  (CallFunction|UpdateUsable))

(event EventOnVisibleChanged
  (params (Character :type Character%20Object%20Reference) (CharacterInteractionComponent :type CIS%20Character%20Interaction%20Component%20Object%20Reference) (InteractionObjectComponent :type CIS%20Interaction%20Object%20Component%20Object%20Reference) (bEnter :type Boolean))
  (bind _asbp_base_interact_object (Utilities|Casting|CastToBP_BaseInteractObject (Components|GetOwner InteractionObjectComponent)))
  (Default|Visible (Default|GetInteractionWidget _asbp_base_interact_object) bEnter))

(event EventOnInitialized
  (params (InteractionCharacter :type Character%20Object%20Reference) (CharacterInteractionComponent :type CIS%20Character%20Interaction%20Component%20Object%20Reference) (InteractionObjectComponent :type CIS%20Interaction%20Object%20Component%20Object%20Reference))
  (EventDispatchers|AssignOnBestObjectforUseChangedDelegate CharacterInteractionComponent (delegate Custom|OnBestObjectForUseChangedDelegate_Event)))

(event EventOnOverlapped
  (params (InteractionCharacter :type Character%20Object%20Reference) (CharacterInteractionComponent :type CIS%20Character%20Interaction%20Component%20Object%20Reference) (InteractionObjectComponent :type CIS%20Interaction%20Object%20Component%20Object%20Reference) (bOverlap :type Boolean))
  (bind _asbp_base_interact_object (Utilities|Casting|CastToBP_BaseInteractObject (Components|GetOwner (Variables|Default|GetCachedInteractionObjectComponent))))
  (Components|Activation|SetActive (Variables|/Game/CharacterInteraction/Blueprints/InteractionObjects/BP_BaseInteractObject.BP_BaseInteractObject_C|GetInteractionWidget _asbp_base_interact_object) bOverlap false))