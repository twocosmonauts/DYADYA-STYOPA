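; Interaction object condition that passes only when nothing blocks the line between an interaction object and the interacting character.
; CheckCondition runs a complex Visibility line trace from the object owner's location to the character's location, each raised by its own vertical offset.
; Both actors are ignored, and the condition returns true when the trace has no blocking hit.
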(fn CheckCondition
  (params (InteractionCharacter :type Character%20Object%20Reference) (CharacterInteractionComponent :type CIS%20Character%20Interaction%20Component%20Object%20Reference) (InteractionObjectComponent :type CIS%20Interaction%20Object%20Component%20Object%20Reference) (InteractionObjectSide :type CIS%20Interaction%20Object%20Side%20Structure%20%28by%20ref%29))
  (bind _returnvalue (Components|GetOwner InteractionObjectComponent))
  (bind _outhit (Collision|LineTraceByChannel self (+ (Transformation|GetActorLocation _returnvalue) (Math|Vector|MakeVector 0.0 0.0 (Variables|Settings|GetObjectTraceVerticalOffset))) (+ (Transformation|GetActorLocation InteractionCharacter) (Math|Vector|MakeVector 0.0 0.0 (Variables|Settings|GetCharacterTraceVerticalOffset))) "TraceTypeQuery1" true (Utilities|Array|MakeArray InteractionCharacter _returnvalue) "None"))
  (return (not (.bBlockingHit (Collision|BreakHitResult _outhit)))))