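; Code lock interaction object that gives visual feedback when it is opened.
; On a state change from its CISInteractionObject to the CIS.CodeLock.Opened state, it tints the lock mesh green through a material Color parameter and shows "OPEN" on its text render.
; A SetText event lets other logic write any value to that text display.
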(event OnObjectStateChangedDelegate(CISInteractionObject)
  (params (NewState :type Gameplay%20Tag%20Structure))
  (if (== "(TagName=\"CIS.CodeLock.Opened\")" NewState)
    (Rendering|Material|SetVectorParameterValueonMaterials (Variables|Default|GetCodeLockMesh) "Color" (Math|Conversions|ToVector(LinearColor) (Class|KismetMathLibrary|LinearColorGreen)))
    (Rendering|Components|TextRender|SetText (Variables|Default|GetTextRender) (Utilities|Text|MakeLiteralText "OPEN"))))

(event Custom|SetText
  (params (Value :type Text%20%28by%20ref%29))
  (Rendering|Components|TextRender|SetText (Variables|Default|GetTextRender) Value))

(fn ConstructionScript)