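; BP_InteractionDoorWithoutAnim is an interactable door that swings open and closed by rotating its DoorRig component with a timeline.
; Object state changes from CISInteractionObject play the timeline for the Opened tag and reverse it for Closed, at a rate set by Duration.
; The door ignores Pawn collision while moving and blocks again when the timeline finishes.
; At BeginPlay the interaction widget snaps to the door's socket.
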(event OnObjectStateChangedDelegate(CISInteractionObject)
  (params (NewState :type Gameplay%20Tag%20Structure))
  (Components|Timeline|SetPlayRate (Variables|Default|GetT_OpenCloseDoor) (/ 1.0 (Variables|Default|GetDuration)))
  (Collision|SetCollisionResponsetoChannel (Variables|Default|GetDoor_Rig) "ECC_Pawn" "ECR_Ignore")
  (|SwitchGameplayTag NewState
    (:CIS.Object.Door.Opened
      (bind _newtrack_0 (Timeline|T_OpenCloseDoor Play)
        (:Update
          (Transformation|SetRelativeRotation (Variables|Default|GetDoor_Rig) (Math|Rotator|MakeRotator 0.0 0.0 _newtrack_0) false false))
        (:Finished
          (Collision|SetCollisionResponsetoChannel (Variables|Default|GetDoor_Rig) "ECC_Pawn" "ECR_Block"))))
    (:CIS.Object.Door.Closed
      (Timeline|T_OpenCloseDoor Reverse))))

(event EventBeginPlay
  (|CallParentFunction)
  (Transformation|AttachComponentToComponent (Variables|Default|GetInteractionWidget) (Variables|Default|GetDoor_Rig) "SM_DoorSocket" "SnapToTarget" "KeepWorld" "KeepWorld" true))

(event Collision|EventActorBeginOverlap
  (params (OtherActor :type Actor%20Object%20Reference))
  (|CallParentFunction OtherActor) ; This node is disabled and will not be called.\nDrag off pins to build functionality.
)

(event EventTick
  (params (DeltaSeconds :type Float%20%28single-precision%29))
  (|CallParentFunction DeltaSeconds) ; This node is disabled and will not be called.\nDrag off pins to build functionality.
)

(fn ConstructionScript
  (|CallParentFunction))