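; BP_CodeLock is an interactable keypad lock: the player moves a highlight with WASD, clicks to enter keys and presses E to leave.
; Entered keys show on a text display; a full-length code matching Password turns the mesh green, fires the opened dispatcher and sets a gameplay-tag state, while mismatches briefly show an error.
; The locally controlled owner acts first, then mirrors selection, display and unlock through server-to-multicast events that other machines apply.
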(event Custom|OnStartUse
  (Variables|Default|SetCurrentIndex 0)
  (Variables|Default|SetSelectedKey 0)
  (Utilities|Array|Clear (Variables|Default|GetCurrentCode))
  (CallFunction|SelectKey 0 false)
  (CallFunction|SetTextonDisplay "" false))

(event Custom|ServerPassMatched
  (CallFunction|MulticastPassMatched))

(event Custom|FinishUsing
  (CallFunction|SelectKey 0 true)
  (CallFunction|SetTextonDisplay "" true)
  (Default|CallDFinishUse))

(event Custom|ServerSelectKey
  (params (ID :type Integer) (Hide :type Boolean))
  (CallFunction|MulticastSelectKey ID Hide))

(event Custom|MulticastSelectKey
  (params (ID :type Integer) (Hide :type Boolean))
  (Utilities|HasAuthority
    (:Not
      (CallFunction|SelectKey ID Hide))))

(event Custom|MulticastSetTextOnDisplay
  (params (Text :type String) (Hide :type Boolean))
  (Utilities|HasAuthority
    (:Not
      (CallFunction|SetTextonDisplay Text Hide))))

(event Custom|ServerSetTextOnDisplay
  (params (Text :type String) (Hide :type Boolean))
  (CallFunction|MulticastSetTextonDisplay Text Hide))

(event Custom|MulticastPassMatched
  (Utilities|HasAuthority
    (:Not
      (CallFunction|PassMatched))))

(event EventBeginPlay
  (|CallParentFunction)
  (Variables|Default|SetKeysMapping (Utilities|Array|MakeArray (Variables|Default|GetBP_CodeLock_1) (Variables|Default|GetBP_CodeLock_2) (Variables|Default|GetBP_CodeLock_3) (Variables|Default|GetBP_CodeLock_4) (Variables|Default|GetBP_CodeLock_5) (Variables|Default|GetBP_CodeLock_6) (Variables|Default|GetBP_CodeLock_7) (Variables|Default|GetBP_CodeLock_8) (Variables|Default|GetBP_CodeLock_9) (Variables|Default|GetBP_CodeLock_Reset) (Variables|Default|GetBP_CodeLock_0))))

(event Input|KeyboardEvents|E
  (params (Key :type Key%20Structure :default "None"))
  (:Pressed
    (CallFunction|FinishUsing)))

(event Input|KeyboardEvents|D
  (params (Key :type Key%20Structure :default "None"))
  (:Pressed
    (bind (_validdirection _id) (CallFunction|DetermineKeyID "NewEnumerator3"))
    (if _validdirection
      (CallFunction|SelectKey _id false))))

(event Input|KeyboardEvents|W
  (params (Key :type Key%20Structure :default "None"))
  (:Pressed
    (bind (_validdirection _id) (CallFunction|DetermineKeyID "NewEnumerator0"))
    (if _validdirection
      (CallFunction|SelectKey _id false))))

(event Input|KeyboardEvents|S
  (params (Key :type Key%20Structure :default "None"))
  (:Pressed
    (bind (_validdirection _id) (CallFunction|DetermineKeyID "NewEnumerator1"))
    (if _validdirection
      (CallFunction|SelectKey _id false))))

(event Input|KeyboardEvents|A
  (params (Key :type Key%20Structure :default "None"))
  (:Pressed
    (bind (_validdirection _id) (CallFunction|DetermineKeyID "NewEnumerator2"))
    (if _validdirection
      (CallFunction|SelectKey _id false))))

(event Input|MouseEvents|LeftMouseButton
  (params (Key :type Key%20Structure :default "None"))
  (bind _selectedkey (Variables|Default|GetSelectedKey))
  (bind _text (Variables|/Game/CharacterInteraction/Blueprints/InteractionObjects/BP_CodeLockKey.BP_CodeLockKey_C|GetText _selectedkey))
  (:Pressed
    (if (not (Variables|Default|GetBlockTextInput))
      (switch string _text
        (:Default
          (if (< (Utilities|Array|Length (Variables|Default|GetCurrentCode)) (Utilities|String|Len (Variables|Default|GetPassword)))
            (Utilities|Array|Add (Variables|Default|GetCurrentCode) _text)
            (if (== (Utilities|Array|Length (Variables|Default|GetCurrentCode)) (Utilities|String|Len (Variables|Default|GetPassword)))
              (if (CallFunction|CheckPass)
                (CallFunction|PassMatched)
                (CallFunction|FinishUsing)
                (else
                  (Variables|Default|SetBlockTextInput true)
                  (CallFunction|SetTextonDisplay "Error" false)
                  (Utilities|FlowControl|Delay 1.5)
                  (CallFunction|SetTextonDisplay "" false)
                  (Variables|Default|SetBlockTextInput false)
                  (Utilities|Array|Clear (Variables|Default|GetCurrentCode))))
              (else
                (CallFunction|SetTextonDisplay (CallFunction|GetCurrentTextonDisplay) false)))))
        (:Remove
          (Utilities|Array|RemoveIndex (Variables|Default|GetCurrentCode) (Utilities|Array|LastIndex (Variables|Default|GetCurrentCode)))
          (CallFunction|SetTextonDisplay (CallFunction|GetCurrentTextonDisplay) false))))))

(fn ConstructionScript)

(fn SelectKey
  (params (Index :type Integer) (Hide :type Boolean))
  (Utilities|FlowControl|Sequence
    (:then_0
      (if Hide
        (Rendering|SetVisibility (Variables|Default|GetCurrentKey) false false)
        (else
          (Variables|Default|SetCurrentIndex Index)
          (Rendering|SetVisibility (Variables|Default|GetCurrentKey) true false)
          (Variables|Default|SetSelectedKey (Utilities|Array|Get(acopy) (Variables|Default|GetKeysMapping) (Variables|Default|GetCurrentIndex)))
          (Transformation|SetWorldLocation (Variables|Default|GetCurrentKey) (Transformation|GetWorldLocation (Utilities|Array|Get(acopy) (Variables|Default|GetKeysMapping) (Variables|Default|GetCurrentIndex))) false false))))
    (:then_1
      (Utilities|HasAuthority
        (:Yes
          (CallFunction|ServerSelectKey Index Hide))))))

(fn DetermineKeyID
  (params (FromDIrection :type E_CodeLockMoveType%20Enum :default "NewEnumerator0"))
  (bind _currentindex (Variables|Default|GetCurrentIndex))
  (bind _currentindex_2 (Variables|Default|GetCurrentIndex))
  (bind _currentindex_3 (Variables|Default|GetCurrentIndex))
  (bind _currentindex_4 (Variables|Default|GetCurrentIndex))
  (bind _returnvalue (- _currentindex_2 3))
  (bind _returnvalue_2 (- _currentindex_4 1))
  (bind _returnvalue_3 (+ _currentindex 1))
  (bind _returnvalue_4 (+ _currentindex_3 3))
  (switch Utilities|FlowControl|Switch|SwitchonE_CodeLockMoveType FromDIrection
    (:NewEnumerator0
      (return (>= _returnvalue 0) _returnvalue))
    (:NewEnumerator1
      (return (<= _returnvalue_4 (Utilities|Array|LastIndex (Variables|Default|GetKeysMapping))) _returnvalue_4))
    (:NewEnumerator2
      (return (>= _returnvalue_2 0) _returnvalue_2))
    (:NewEnumerator3
      (return (<= _returnvalue_3 (Utilities|Array|LastIndex (Variables|Default|GetKeysMapping))) _returnvalue_3))))

(fn SetTextonDisplay
  (params (Text :type String) (Hide :type Boolean))
  (LocalVariables|SetfinalText (Class|KismetTextLibrary|TexttoUpper (Utilities|Text|MakeLiteralText (Utilities|Text|ToText(String) Text))))
  (Utilities|FlowControl|Sequence
    (:then_0
      (if Hide
        (if (not (Variables|Default|GetOpened))
          (Rendering|Components|TextRender|SetText (Variables|Default|GetTextRender) (Utilities|Text|ToText(String) "****")))
        (elif (Utilities|Enum|Equal(Enum) Text "")
          (Rendering|Components|TextRender|SetText (Variables|Default|GetTextRender) (Utilities|Text|ToText(String) "****"))
          (else
            (Rendering|Components|TextRender|SetText (Variables|Default|GetTextRender) (LocalVariables|GetfinalText))))))
    (:then_1
      (Utilities|HasAuthority
        (:Yes
          (CallFunction|ServerSetTextonDisplay Text Hide))))))

(fn GetCurrentTextonDisplay
  (for _array_element (Variables|Default|GetCurrentCode)
    (LocalVariables|SetfinalCode (Utilities|String|Append (LocalVariables|GetfinalCode) _array_element)))
  (return (LocalVariables|GetfinalCode)))

(fn CheckPass
  (return (Utilities|Enum|Equal(Enum) (CallFunction|GetCurrentTextonDisplay) (Variables|Default|GetPassword))))

(fn PassMatched
  (if (not (Variables|Default|GetOpened))
    (Variables|Default|SetOpened true)
    (CallFunction|SetTextonDisplay "open" false)
    (Rendering|Material|SetVectorParameterValueonMaterials (Variables|Default|GetCodeLockMesh) "Color" (Math|Conversions|ToVector(LinearColor) (Class|KismetMathLibrary|LinearColorGreen)))
    (Default|CallDOpened)
    (Utilities|HasAuthority
      (:Yes
        (CallFunction|ServerPassMatched)
        (Class|CISInteractionObjectComponent|SetObjectState (Variables|Default|GetCISInteractionObject) (GameplayTags|MakeLiteralGameplayTag "(TagName=\"CIS.CodeLock.Opened\")"))))))