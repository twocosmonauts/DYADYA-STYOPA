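; Bat variant of the melee weapon that adds a reaction to striking actors tagged "Pipe" on top of the parent hit effect.
; A DoOnce reset by a short delay debounces pipe hits into a counter, while a retriggerable delay waits for the hitting to stop.
; It then sends every BPI_Dialog actor an AnswerMessage stating whether the pipe was hit more than once, and clears the count.
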(event EventHitEffect
  (params (IpLoc :type Vector :default "0, 0, 0") (IpNormal :type Vector :default "0, 0, 0") (SurfaceType :type EPhysicalSurface%20Enum :default "SurfaceType_Default"))
  (|CallParentFunction IpLoc IpNormal SurfaceType)
  (for _array_element (Variables|Default|GetHitedActorAry)
    (if (Actor|ActorHasTag _array_element "Pipe")
      (Utilities|FlowControl|Sequence
        (:then_0
          (Utilities|FlowControl|DoOnce false :!label _label
            (:Completed
              (Math|Integer|IncrementInt (Variables|Default|GetHitCount)
                (:%20%20
                  (Utilities|FlowControl|RetriggerableDelay 3.0)
                  (bind _outactors (Actor|GetAllActorswithInterface "/Game/ProjectDyadyaStyopa/BP/BPI_Dialog.BPI_Dialog_C"))
                  (for _array_element_2 _outactors
                    (Class|BPIDialog|Answer(Message) _array_element_2 (> (Variables|Default|GetHitCount) 1)))
                  (Variables|Default|SetHitCount 0))))))
        (:then_1
          (Utilities|FlowControl|Delay 1.0)
          (goto _label Reset))))))

(fn ConstructionScript
  (|CallParentFunction))