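; Base melee weapon Blueprint that detects hits during attacks and hands them to damage processing.
; On BeginPlay it caches its sphere components; between StartCheckCollision and EndCheckCollision, Tick sweeps multi-sphere traces from each saved position to the current one, covering movement between frames.
; It ignores the owner, records each actor once per window, and stops at the first sphere reporting hits each tick.
; A HitEffect event forwards location, normal and surface type to SpawnHitEffect.
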(event EventBeginPlay
  (Variables|Default|SetCollisionAry (Actor|GetComponentsByClass "/Script/Engine.SphereComponent")))

(event EventTick
  (params (DeltaSeconds :type Float%20%28single-precision%29))
  (if (Variables|Default|GetIsCheckCollision)
    (Utilities|Array|Clear (Variables|Default|GetHitAry))
    (bind _result (CallFunction|CheckCollision))
    (for _array_element _result
      (CallFunction|DamageProcess (.HitActor (Collision|BreakHitResult _array_element)) _array_element))))

(event EventHitEffect
  (params (IpLoc :type Vector :default "0, 0, 0") (IpNormal :type Vector :default "0, 0, 0") (SurfaceType :type EPhysicalSurface%20Enum :default "SurfaceType_Default"))
  (CallFunction|SpawnHitEffect IpLoc IpNormal SurfaceType))

(fn ConstructionScript
  (|CallParentFunction))

(fn SaveCollisionPos
  (Utilities|Array|Clear (Variables|Default|GetSaveCollisionPosAry))
  (for _array_element (Variables|Default|GetCollisionAry)
    (Utilities|Array|Add (Variables|Default|GetSaveCollisionPosAry) (Transformation|GetWorldLocation _array_element))))

(fn CheckCollision
  (bind (_array_element _array_index) (Utilities|Array|ForEachLoopwithBreak (Variables|Default|GetCollisionAry) :!label _label)
    (:LoopBody
      (bind (_outhits _returnvalue) (Collision|MultiSphereTraceForObjects (Utilities|Array|Get(acopy) (Variables|Default|GetSaveCollisionPosAry) _array_index) (Transformation|GetWorldLocation _array_element) (Variables|/Script/Engine.SphereComponent|GetSphereRadius _array_element) (Utilities|Array|MakeArray "ObjectTypeQuery1" "ObjectTypeQuery4" "ObjectTypeQuery3") false (Utilities|Array|MakeArray (Components|GetOwner)) "None" true "(R=1.000000,G=0.000000,B=0.000000,A=1.000000)" "(R=0.000000,G=1.000000,B=0.000000,A=1.000000)" 15.0))
      (if _returnvalue
        (for _array_element_2 _outhits
          (if (not (Utilities|Array|ContainsItem (Variables|Default|GetHitedActorAry) (.HitActor (Collision|BreakHitResult _array_element_2))))
            (Utilities|Array|Add (Variables|Default|GetHitedActorAry) (.HitActor (Collision|BreakHitResult _array_element_2)))
            (Utilities|Array|Add (LocalVariables|GetLocalHitAry) _array_element_2)))
        (goto _label Break)))
    (:Completed
      (CallFunction|SaveCollisionPos)
      (return (LocalVariables|GetLocalHitAry)))))

(fn StartCheckCollision
  (Variables|Default|SetIsCheckCollision true)
  (Utilities|Array|Clear (Variables|Default|GetHitedActorAry))
  (CallFunction|SaveCollisionPos)
  (return true))

(fn EndCheckCollision
  (Variables|Default|SetIsCheckCollision false)
  (return true))