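; Base weapon Blueprint for the FPS melee weapon system, with empty fire, reload, collision-check and hit-effect hooks that suggest child weapons supply the behavior.
; DamageProcess makes AI noise, then applies random-range point damage to characters other than the instigator.
; Non-character hits call HitEffect and push physics-simulating components along the inverse hit normal.
; Helpers toggle mesh or bone visibility and spawn impact particles and sound through surface-type selects.
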(event Custom|HitEffect
  (params (IpLoc :type Vector) (IpNormal :type Vector) (SurfaceType :type EPhysicalSurface%20Enum :default "SurfaceType_Default")))

(event Custom|Reload)

(event Custom|Fire
  (params (IpFireTarget :type Vector) (IpBarrelIndex :type Integer) (IpCharSpreadHalfAngleY :type Float%20%28double-precision%29) (IpCharSpreadHalfAngleZ :type Float%20%28double-precision%29)))

(event Custom|StartFire
  (params (IpFireTarget :type Vector) (IpBarrelIndex :type Integer)))

(event Custom|UpdateFireTarget
  (params (IpFireTarget :type Vector) (IpBarrelIndex :type Integer)))

(event Custom|ShowBone
  (params (IsVisible :type Boolean) (IpBoneName :type Name))
  (if (not IsVisible)
    (Components|SkinnedMesh|HideBonebyName (Variables|Default|GetSkeletalMesh) IpBoneName "PBO_None")
    (else
      (Components|SkinnedMesh|UnHideBonebyName (Variables|Default|GetSkeletalMesh) IpBoneName))))

(event Custom|EndFire)

(event Custom|PlayFireAnim)

(event Custom|FireEffect
  (params (BarrelIndex :type Integer)))

(fn ConstructionScript)

(fn Show
  (params (Visible :type Boolean))
  (Utilities|FlowControl|Sequence
    (:then_0
      (Utilities|IsValid (Variables|Default|GetStaticMesh)
        (:Is%20Valid
          (Rendering|SetVisibility (Variables|Default|GetStaticMesh) Visible true))))
    (:then_1
      (Utilities|IsValid (Variables|Default|GetSkeletalMesh)
        (:Is%20Valid
          (Rendering|SetVisibility (Variables|Default|GetSkeletalMesh) Visible true))))))

(fn StartCheckCollision
  (return false))

(fn EndCheckCollision
  (return true))

(fn DamageProcess
  (params (IpHitActor :type Actor%20Object%20Reference) (IpHitResult :type Hit%20Result%20Structure))
  (bind (_bblockinghit _binitialoverlap _time _distance _location _impactpoint _normal) (Collision|BreakHitResult IpHitResult))
  (bind (_bblockinghit_2 _binitialoverlap_2 _time_2 _distance_2 _location_2 _impactpoint_2 _normal_2 _impactnormal _physmat _hitactor _hitcomponent) (Collision|BreakHitResult IpHitResult))
  (Utilities|FlowControl|Sequence
    (:then_0
      ;[0.03125 1 0] Make Noise
      (Class|Actor|MakeNoise 1.0 (Variables|Actor|GetInstigator) (Transformation|GetActorLocation) 2e+02 "None")
      ;[0.4062 0 1] Check if can take damage
      (Utilities|Casting|CastToBP_BaseChar IpHitActor
        (:then
          (if (!= IpHitActor (Game|GetInstigator))
            (LocalVariables|SetLocalDamage (Math|Random|RandomFloatinRange (Variables|NonEditable|GetMinDamage) (Variables|NonEditable|GetMaxDamage)))
            ;[0.875 0 1] Apply Point Damage
            (Game|Damage|ApplyPointDamage IpHitActor (LocalVariables|GetLocalDamage) (Math|Rotator|GetRotationXVector (Transformation|GetActorRotation)) IpHitResult 0 (Game|GetInstigator))))
        (:CastFailed
          ;[1 0.09375 0] Hit effect
          (CallFunction|HitEffect _location _normal (Collision|GetSurfaceType IpHitResult))
          (if (Physics|IsSimulatingPhysics _hitcomponent "None")
            (Physics|AddImpulseatLocation _hitcomponent (* _normal_2 -5e+04) _location_2 "None")))))
    (:then_1
      (return false))))

(fn SpawnHitEffect
  (params (IpHitLoc :type Vector) (IpHitNormal :type Vector) (IpSurfaceType :type EPhysicalSurface%20Enum :default "SurfaceType_Default"))
  (bind _returnvalue (Math|Conversions|RotationFromXVector IpHitNormal))
  (bind (_roll _pitch _yaw) (Math|Rotator|BreakRotator _returnvalue))
  ;[1 0 0.3281] Spawn Eimmter
  (Effects|SpawnEmitteratLocation (Utilities|Select :Index IpSurfaceType :SurfaceType_Default "/Game/FPSMeleeWeaponSystem/Particles/PS_Impact_Default.PS_Impact_Default") IpHitLoc (Math|Rotator|MakeRotator _roll (+ _pitch -9e+01) _yaw))
  ;[0.6875 0 1] Play hit sound
  (Audio|PlaySoundatLocation (Utilities|Select :Index IpSurfaceType :SurfaceType_Default "/Game/FPSMeleeWeaponSystem/Audios/Cues/Weapons/Melee_ConcreteHit2_Cue.Melee_ConcreteHit2_Cue") IpHitLoc "0, 0, 0" 1.0 1.0 0.0 "/Game/FPSMeleeWeaponSystem/Audios/WeaponImpactSoundAttenuation.WeaponImpactSoundAttenuation" 0 0 0))