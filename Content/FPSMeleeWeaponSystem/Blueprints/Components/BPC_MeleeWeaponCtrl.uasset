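; Actor component that manages a first-person character's melee weapons, handling attacks, switching and unequipping.
; Spawns each configured weapon attached to an Arms socket, toggles visibility on selection, and destroys them at EndPlay.
; Attack and switch are mutually locked, timed by Delays using lengths returned from Arms AnimInstance messages; switching also applies per-weapon arm offsets.
; Anim notify events start and end collision checks on the current weapon.
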(event Custom|StartChangeWeapon
  (params (InTargetWeaponIndex :type Integer))
  (bind _meleeweaponinfoary (Variables|Default|GetMeleeWeaponInfoAry))
  (bind _curselectweaponindex (Variables|Default|GetCurSelectWeaponIndex))
  (bind _originarmsrot (Variables|Default|GetOriginArmsRot))
  (bind (_roll _pitch _yaw) (Math|Rotator|BreakRotator _originarmsrot))
  (bind _output (Utilities|Array|Get(acopy) _meleeweaponinfoary _curselectweaponindex))
  (bind _offsetrot (Utilities|Struct|BreakS_FPS_MeleeWeaponInfo _output))
  (bind (_roll_2 _pitch_2 _yaw_2) (Math|Rotator|BreakRotator _offsetrot))
  ;[1 0.5625 0] StartChangeWeapon
  (if (Math|Boolean|ANDBoolean (not (Variables|Default|GetIsMeleeAttack)) (not (Variables|Default|GetIsChangingWeapon)) (!= InTargetWeaponIndex (Variables|Default|GetCurSelectWeaponIndex)))
    (Variables|Default|SetIsChangingWeapon true)
    (bind _result (Class|FPSMeleeArmAnimInterface|PlayUnEquipAnim(Message) (Components|SkeletalMesh|GetAnimInstance (Variables|Default|GetArms))))
    (Utilities|FlowControl|Delay _result)
    (CallFunction|SelectWeapon InTargetWeaponIndex)
    (Transformation|SetRelativeRotation (Variables|Default|GetArms) (Math|Rotator|MakeRotator (+ _roll _roll_2) (+ _pitch _pitch_2) (+ _yaw _yaw_2)) false false)
    (Transformation|SetRelativeLocation (Variables|Default|GetArms) (+ (Variables|Default|GetOriginArmsLoc) (Utilities|Struct|BreakS_FPS_MeleeWeaponInfo (Utilities|Array|Get(acopy) (Variables|Default|GetMeleeWeaponInfoAry) (Variables|Default|GetCurSelectWeaponIndex)))) false false)
    (bind _result_2 (Class|FPSMeleeArmAnimInterface|GetEquipAnimLength(Message) (Components|SkeletalMesh|GetAnimInstance (Variables|Default|GetArms))))
    (Utilities|FlowControl|Delay _result_2)
    (Variables|Default|SetIsChangingWeapon false)))

(event Custom|StartFireMeleeWeapon
  (params (Owner :type BP%20CIS%20Character%20Object%20Reference))
  (bind _arms (Variables|Default|GetArms)
    (:then
      (if (and (not (Variables|Default|GetIsMeleeAttack)) (not (Variables|Default|GetIsChangingWeapon)))
        (Variables|Default|SetIsMeleeAttack true)
        (bind _result (Class|FPSMeleeArmAnimInterface|PlayMeleeAttackAnim(Message) (Components|SkeletalMesh|GetAnimInstance _arms)))
        ;[0.7344 0 1] Starting MeleeAttack
        (Utilities|FlowControl|Delay _result)
        (Variables|Default|SetIsMeleeAttack false)
        (Default|EndMeleeAttack Owner)))
    (:else)))

(event EventBeginPlay
  ;[0.4766 1 0] Event - BeginPlay
  (|CallParentFunction)
  (CallFunction|CreateAllWeapons))

(event EventEndPlay
  (params (EndPlayReason :type EEndPlayReason%20Enum :default "Destroyed"))
  ;[0 0.8828 1] Event - EndPlay
  (CallFunction|DestoryAllWeapons))

(event EventAnimNotifyonAnimStartCheckMeleeCollision
  ;[0.4766 0 1] AnimNotify -StartCheckMeleeCollision, EndCheckMeleeCollision
  (Default|StartCheckCollision (Variables|Default|GetCurWeapon)))

(event EventAnimNotifyonAnimEndCheckMeleeCollision
  ;[0.4766 0 1] AnimNotify -StartCheckMeleeCollision, EndCheckMeleeCollision
  (Default|EndCheckCollision (Variables|Default|GetCurWeapon)))

(fn CreateAllWeapons
  (bind _ownerplayerchar (Variables|Default|GetOwnerPlayerChar))
  (for (_array_element _array_index) (Variables|Default|GetMeleeWeaponInfoAry)
    (LocalVariables|SetLocalIndex _array_index)
    (if (Utilities|IsValidClass (.WeaponClass (Utilities|Struct|BreakS_FPS_MeleeWeaponInfo _array_element)))
      (bind _returnvalue (Game|SpawnActorfromClass (.WeaponClass (Utilities|Struct|BreakS_FPS_MeleeWeaponInfo _array_element)) (Transformation|GetActorTransform (Variables|Default|GetOwnerPlayerChar)) "Undefined" "SelectDefaultAtRuntime" _ownerplayerchar _ownerplayerchar))
      (Transformation|AttachComponentToComponent _returnvalue (Variables|Default|GetArms) (.AttachSocketName (Utilities|Struct|BreakS_FPS_MeleeWeaponInfo _array_element)) "SnapToTarget" "SnapToTarget" "SnapToTarget" true)
      (Rendering|SetActorHiddenInGame _returnvalue true)
      (Utilities|Struct|SetmembersinS_FPS_MeleeWeaponInfo (Utilities|Array|Get(acopy) (Variables|Default|GetMeleeWeaponInfoAry) (LocalVariables|GetLocalIndex)) _returnvalue))))

(fn SelectWeapon
  (params (InSelectWeaponIndex :type Integer))
  (Variables|Default|SetCurSelectWeaponIndex InSelectWeaponIndex)
  (CallFunction|HideAllWeapons false)
  (if (> (Variables|Default|GetCurSelectWeaponIndex) -1)
    (Rendering|SetActorHiddenInGame (.WeaponRef (Utilities|Struct|BreakS_FPS_MeleeWeaponInfo (Utilities|Array|Get(acopy) (Variables|Default|GetMeleeWeaponInfoAry) (Variables|Default|GetCurSelectWeaponIndex)))) false)
    (Variables|Default|SetCurWeapon (.WeaponRef (Utilities|Struct|BreakS_FPS_MeleeWeaponInfo (Utilities|Array|Get(acopy) (Variables|Default|GetMeleeWeaponInfoAry) (Variables|Default|GetCurSelectWeaponIndex)))))))

(fn HideAllWeapons
  (params (bNewHidden :type Boolean))
  (for _array_element (Variables|Default|GetMeleeWeaponInfoAry)
    (Rendering|SetActorHiddenInGame (.WeaponRef (Utilities|Struct|BreakS_FPS_MeleeWeaponInfo _array_element)) bNewHidden)))

(fn InitARMS
  (params (InArm :type Skeletal%20Mesh%20Component%20Object%20Reference))
  (bind _output_get (Variables|Default|SetArms InArm))
  (Variables|Default|SetOriginArmsLoc (Variables|/Script/Engine.SceneComponent|GetRelativeLocation _output_get))
  (Variables|Default|SetOriginArmsRot (Variables|/Script/Engine.SceneComponent|GetRelativeRotation _output_get))
  (CallFunction|CreateAllWeapons))

(fn DestoryAllWeapons
  (for _array_element (Variables|Default|GetMeleeWeaponInfoAry)
    (Utilities|IsValid (.WeaponRef (Utilities|Struct|BreakS_FPS_MeleeWeaponInfo _array_element))
      (:Is%20Valid
        (Actor|DestroyActor (.WeaponRef (Utilities|Struct|BreakS_FPS_MeleeWeaponInfo _array_element)))))))

(fn UnEquip
  (CallFunction|SelectWeapon -1)
  (Transformation|SetRelativeRotation (Variables|Default|GetArms) (Variables|Default|GetOriginArmsRot) false false)
  (Transformation|SetRelativeLocation (Variables|Default|GetArms) (Variables|Default|GetOriginArmsLoc) false false)
  (CallFunction|HideAllWeapons false))

(fn IsSelectWeapon
  (return (> (Variables|Default|GetCurSelectWeaponIndex) -1)))

(fn GetEquipAnimLength
  (return 0.0))

(fn PlayMeleeAttackAnim
  (params (Index :type Integer))
  (return 0.0))

(fn PlayUnEquipAnim
  (return 0.0))