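; First-person player character Blueprint for a melee weapon system, handling movement, look, jump, crouch, sprint and weapon input.
; On BeginPlay it caches the walk speed, initializes the melee weapon controller component with the arm and selects the first weapon.
; Fire and number keys delegate attacks and weapon switching to that component.
; Tick polls sprint state, allowing sprint only while moving forward and not falling, by swapping max walk speed.
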(event EventBeginPlay
  (bind _bpc_meleeweaponctrl (Variables|Default|GetBPC_MeleeWeaponCtrl))
  ;[1 0 0.3047] Event - BeginPlay
  (|CallParentFunction)
  ;;[0 0.6016 1] Set Character Movement Walk Speed
  (Variables|FPSMeleeWeaponSystem|SetOriginWalkSpeed (Variables|/Script/Engine.CharacterMovementComponent|GetMaxWalkSpeed (Variables|Character|GetCharacterMovement)))
  (Default|InitARMS _bpc_meleeweaponctrl (Variables|Default|GetArm))
  (Default|SelectWeapon _bpc_meleeweaponctrl))

(event EventTick
  (params (DeltaSeconds :type Float%20%28single-precision%29))
  ;[1 0.6797 0] Tick
  (CallFunction|TickSprint))

(fn ConstructionScript)

(event Input|ActionEvents|InputActionFire
  (params (Key :type Key%20Structure))
  ;[1 0 0.7969] Action Fire
  (:Pressed
    (Default|StartFireMeleeWeapon (Variables|Default|GetBPC_MeleeWeaponCtrl))))

(event Input|ActionEvents|InputActionCrouch
  (params (Key :type Key%20Structure))
  ;[0 1 0.9766] Action Crouch
  (:Pressed
    (if (not (Variables|Default|GetbIsCrouched))
      (if (not (AI|Components|NavMovement|IsFalling (Variables|Character|GetCharacterMovement)))
        (CallFunction|ReleasedSprintInput)
        (Character|Crouch))
      (else
        (Character|UnCrouch)))))

(event Input|ActionEvents|InputActionJump
  (params (Key :type Key%20Structure))
  ;[0 1 0.5078] Action Jump
  (:Pressed
    (Character|UnCrouch)
    (Character|Jump))
  (:Released
    (Character|StopJumping)))

(event Input|ActionEvents|InputActionSprint
  (params (Key :type Key%20Structure))
  ;[0.3828 0 1] Action Sprint
  (:Pressed
    (Variables|FPSMeleeWeaponSystem|SetIsPressingSprintInput true))
  (:Released
    (Variables|FPSMeleeWeaponSystem|SetIsPressingSprintInput false)))

(event Input|AxisEvents|InputAxisTurn
  (params (AxisValue :type Float%20%28single-precision%29))
  ;[0 0.6484 1] Axis Turn, LookUp
  (Pawn|Input|AddControllerYawInput AxisValue))

(event Input|AxisEvents|InputAxisLookUp
  (params (AxisValue :type Float%20%28single-precision%29))
  ;[0 0.6484 1] Axis Turn, LookUp
  (Pawn|Input|AddControllerPitchInput AxisValue))

(event Input|AxisEvents|InputAxisMoveForward
  (params (AxisValue :type Float%20%28single-precision%29))
  ;[0.7812 1 0] Axis Move Forward, Right
  (Variables|FPSMeleeWeaponSystem|SetAxisMoveForwardValue AxisValue)
  (Pawn|Input|AddMovementInput (Math|Vector|GetForwardVector (Math|Rotator|MakeRotator 0.0 0.0 (.Yaw (Math|Rotator|BreakRotator (Transformation|GetWorldRotation (Variables|Default|GetCamera)))))) (Variables|FPSMeleeWeaponSystem|GetAxisMoveForwardValue) false))

(event Input|AxisEvents|InputAxisMoveRight
  (params (AxisValue :type Float%20%28single-precision%29))
  ;[0.7812 1 0] Axis Move Forward, Right
  (Variables|FPSMeleeWeaponSystem|SetAxisMoveRightValue AxisValue)
  (Pawn|Input|AddMovementInput (Math|Vector|GetRightVector (Math|Rotator|MakeRotator 0.0 0.0 (.Yaw (Math|Rotator|BreakRotator (Transformation|GetWorldRotation (Variables|Default|GetCamera)))))) (Variables|FPSMeleeWeaponSystem|GetAxisMoveRightValue) false))

(event Input|KeyboardEvents|2
  (params (Key :type Key%20Structure))
  ;[1 0.04688 0] Action Number
  (:Pressed
    (Default|StartChangeWeapon (Variables|Default|GetBPC_MeleeWeaponCtrl) 1)))

(event Input|KeyboardEvents|1
  (params (Key :type Key%20Structure))
  ;[1 0.04688 0] Action Number
  (:Pressed
    (Default|StartChangeWeapon (Variables|Default|GetBPC_MeleeWeaponCtrl))))

(event Custom|TickSprint
  ;[1 1 1] Check if player pressed sprint input
  (if (Variables|FPSMeleeWeaponSystem|GetIsPressingSprintInput)
    ;[1 1 1] Check varibles if Player can sprint, start sprint if player can.
    (if (> (Variables|FPSMeleeWeaponSystem|GetAxisMoveForwardValue) 0.0)
      (if (not (Variables|Default|GetIsSprint))
        ;[1 1 1] check if character is falling and player character state is default.
        (if (not (AI|Components|NavMovement|IsFalling (Variables|Character|GetCharacterMovement)))
          (CallFunction|StartSprint))
        (else
          ;[1 1 1] if IsSprint is true and isfalling is true, stop sprinting
          (if (AI|Components|NavMovement|IsFalling (Variables|Character|GetCharacterMovement))
            (CallFunction|StopSprint))))
      (else
        ;[1 1 1] Stop sprint if player character is sprinting.
        (if (Variables|Default|GetIsSprint)
          (CallFunction|StopSprint))))
    (else
      ;[1 1 1] Stop sprint if player character is sprinting
      (if (Variables|Default|GetIsSprint)
        (CallFunction|StopSprint)))))

(event Custom|Released_SprintInput
  ;[1 1 1] Sprint Inputs
)

(event Custom|Pressed_SprintInput
  ;[1 1 1] Sprint Inputs
)

(event Custom|Start_Sprint
  ;[1 1 1] Start Sprint
  (Variables|Default|SetIsSprint true)
  (Variables|/Script/Engine.CharacterMovementComponent|SetMaxWalkSpeed (Variables|Character|GetCharacterMovement) (Variables|FPSMeleeWeaponSystem|GetSprintMaxWalkSpeed))
  (Animation|StopAnimMontage 0))

(event Custom|Stop_Sprint
  ;[1 1 1] Stop Sprint
  (Variables|Default|SetIsSprint false)
  (Variables|/Script/Engine.CharacterMovementComponent|SetMaxWalkSpeed (Variables|Character|GetCharacterMovement) (Variables|FPSMeleeWeaponSystem|GetOriginWalkSpeed)))